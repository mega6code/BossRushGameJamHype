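; Boss actor that reuses a single static mesh actor to play three snowman bosses (white, blue, red) in turn.
; StartLoop begins the cycle, and WhichBoss swaps the mesh and moves the actor to a fight pad's EnemyPos.
; The first boss uses the first pad found, while the others look pads up by tag.
; BossSwitch polls IsAlive on a short delay, advancing on death while the first-found pad's Loop is set, wrapping after the third.
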(event `PadRef`
  (bind _outactors (`GameplayStatics.GetAllActorsOfClass` "/Game/Bosses/Blueprints/BP_FightPad.BP_FightPad_C"))
  (set `self.FightPadRef` (`|GetArrayItem` _outactors)))

(event `self.ReceiveBeginPlay`
  (`self.PadRef`))

(event `StartLoop`
  (set `self.IsAlive` true)
  (set `self.IsAlive2` true)
  (`self.Boss Switch`))

(event `Boss Switch`
  (if (== (`self.CurrentBoss`) 3) :!label _label
    (set `self.CurrentBoss` 0)
    (set `self.IsAlive` true)
    (set `self.IsAlive2` true)
    (goto _label)
    (else
      (set `self.CurrentBoss` (+ (`self.CurrentBoss`) 1))
      (`self.Which Boss`)
      (`KismetSystemLibrary.RetriggerableDelay` 0.2 :!label _label_2)
      (if (`self.IsAlive`)
        (goto _label_2)
        (elif (`/Game/Bosses/Blueprints/BP_FightPad.Loop` (`self.FightPadRef`))
          (set `self.IsAlive` true)
          (`self.Boss Switch`))))))

(event `Which Boss`
  (bind (_returnvalue_x _returnvalue_y) (`KismetMathLibrary.BreakVector` (`SceneComponent.K2_GetComponentLocation` (`/Game/Bosses/Blueprints/BP_FightPad.EnemyPos` (`self.FightPadRef`)))))
  ; Fight Switch
  (if (== (`self.CurrentBoss`) 1)
    (`StaticMeshComponent.SetStaticMesh` (`self.StaticMesh`) "/Game/Bosses/Meshes/WhiteSnowmanBoss.WhiteSnowmanBoss")
    (`self.K2_SetActorLocation` (`KismetMathLibrary.MakeVector` _returnvalue_x _returnvalue_y 70.0))
    (elif (== (`self.CurrentBoss`) 2)
      (`StaticMeshComponent.SetStaticMesh` (`self.StaticMesh`) "/Game/Bosses/Meshes/BlueSnowmanBoss.BlueSnowmanBoss")
      (bind _outactors (`GameplayStatics.GetAllActorsOfClassWithTag` "/Game/Bosses/Blueprints/BP_FightPad.BP_FightPad_C" "Boss 2"))
      (bind (_returnvalue_x_2 _returnvalue_y_2) (`KismetMathLibrary.BreakVector` (`SceneComponent.K2_GetComponentLocation` (`/Game/Bosses/Blueprints/BP_FightPad.EnemyPos` (`|GetArrayItem` _outactors)))))
      (`self.K2_SetActorLocation` (`KismetMathLibrary.MakeVector` _returnvalue_x_2 _returnvalue_y_2 70.0))
      (else
        (`StaticMeshComponent.SetStaticMesh` (`self.StaticMesh`) "/Game/Bosses/Meshes/RedSnowmanBoss.RedSnowmanBoss")
        (bind _outactors_2 (`GameplayStatics.GetAllActorsOfClassWithTag` "/Game/Bosses/Blueprints/BP_FightPad.BP_FightPad_C" "Boss 3"))
        (bind (_returnvalue_x_3 _returnvalue_y_3) (`KismetMathLibrary.BreakVector` (`SceneComponent.K2_GetComponentLocation` (`/Game/Bosses/Blueprints/BP_FightPad.EnemyPos` (`|GetArrayItem` _outactors_2)))))
        (`self.K2_SetActorLocation` (`KismetMathLibrary.MakeVector` _returnvalue_x_3 _returnvalue_y_3 70.0))))))

(fn `UserConstructionScript`)