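; BP_Wheel is a one-use fortune wheel that spins on any actor overlap and grants a bonus to either the boss or the player jet.
; A timeline pitches the mesh by a random one-to-two-turn angle, then a delayed loop matches that angle to a segment in the Degree array.
; The segment index selects boss health, jet stamina or jet health boosts before the wheel resets and destroys itself.
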(event `self.ReceiveBeginPlay`
  (bind _outactors (`GameplayStatics.GetAllActorsOfClass` "/Game/Jet/BluePrints/BP_Jet.BP_Jet_C"))
  (set `self.JetRef` (`|GetArrayItem` _outactors))
  (bind _outactors_2 (`GameplayStatics.GetAllActorsOfClass` "/Game/Bosses/Blueprints/BP_Boss.BP_Boss_C"))
  (set `self.BossRef` (`|GetArrayItem` _outactors_2)))

(event `Which Number Check`
  (bind _bossref (`self.BossRef`))
  (bind _jetref (`self.JetRef`))
  (bind _jetref_2 (`self.JetRef`))
  (bind _returnvalue (* (`/Game/Bosses/Blueprints/BP_Boss.MaxHealth` _bossref) 1.5))
  (bind _returnvalue_2 (* (`/Game/Jet/BluePrints/BP_Jet.MaxStamina` _jetref_2) 1.5))
  (bind _returnvalue_3 (* (`/Game/Jet/BluePrints/BP_Jet.MaxHealth` _jetref) 1.5))
  ; Which powerup
  (if (or (== (`self.DegreeIncrease`) 0) (== (`self.DegreeIncrease`) 2) (== (`self.DegreeIncrease`) 4) (== (`self.DegreeIncrease`) 6))
    (`KismetSystemLibrary.PrintString` "BONUS HEALTH FOR BOSS")
    (set `/Game/Bosses/Blueprints/BP_Boss.MaxHealth` _returnvalue _bossref)
    (set `/Game/Bosses/Blueprints/BP_Boss.CurrentHealth` _returnvalue _bossref)
    (elif (or (== (`self.DegreeIncrease`) 1) (== (`self.DegreeIncrease`) 5))
      (`KismetSystemLibrary.PrintString` "BOSS STAMINA FOR PLAYER")
      (set `/Game/Jet/BluePrints/BP_Jet.Stamina` _returnvalue_2 _jetref_2)
      (set `/Game/Jet/BluePrints/BP_Jet.MaxStamina` _returnvalue_2 _jetref_2)
      (elif (or (== (`self.DegreeIncrease`) 3) (== (`self.DegreeIncrease`) 7))
        (`KismetSystemLibrary.PrintString` "BONUS HEALTH FOR PLAYER")
        (set `/Game/Jet/BluePrints/BP_Jet.BaseHealth` _returnvalue_3 _jetref)
        (set `/Game/Jet/BluePrints/BP_Jet.MaxHealth` _returnvalue_3 _jetref)))))

(event `self.ReceiveActorBeginOverlap`
  (params (OtherActor :type "Actor Object Reference"))
  ; Spinning the wheel
  (if (not (`self.IsSpinning`))
    (set `self.RandomNumber` (`KismetMathLibrary.RandomFloatInRange` 360.0 720.0))
    (bind (_direction _rotation) (`Timeline|SpinningAnimation` :!via `PlayFromStart`)
      (:`Update`
        (set `self.IsSpinning` true)
        (`SceneComponent.K2_SetWorldRotation` (`self.StaticMesh`) (`KismetMathLibrary.MakeRotator` 0.0 (* _rotation (`self.RandomNumber`))) false false))
      (:`Finished`
        (set `self.RandomNumber` (- (`self.RandomNumber`) 360.0))
        (if (and (> (`self.RandomNumber`) (`|GetArrayItem` (`self.Degree`) (`self.DegreeIncrease`))) (<= (`self.RandomNumber`) (`|GetArrayItem` (`self.Degree`) (+ (`self.DegreeIncrease`) 1)))) :!label _label
          (`self.Which Number Check`)
          (set `self.DegreeIncrease` 0)
          (set `self.RandomNumber` 0.0)
          (`KismetSystemLibrary.Delay` 1.0)
          (`SceneComponent.K2_SetWorldRotation` (`self.StaticMesh`) (`KismetMathLibrary.MakeRotator` 0.0) false false)
          (set `self.IsSpinning` false)
          (`self.K2_DestroyActor`)
          (else
            (set `self.DegreeIncrease` (+ (`self.DegreeIncrease`) 1))
            (`KismetSystemLibrary.RetriggerableDelay` 0.1)
            (goto _label)))))))

(fn `UserConstructionScript`)