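; BP_CamPos is an actor that moves itself to the camera position of the fight pad matching the current boss.
; From BeginPlay, MoveCamera loops on a 0.2-second retriggerable delay, reading CurrentBoss from the first BP_Boss.
; It teleports to that pad's CameraPos with CamRot rotation.
; Boss 1 uses the first BP_FightPad found, while later bosses use pads tagged "Boss 2" or "Boss 3".
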(event `self.ReceiveBeginPlay`
  (`self.MoveCamera`))

(event `MoveCamera`
  (bind _camrot (`self.CamRot`))
  (bind _outactors (`GameplayStatics.GetAllActorsOfClass` "/Game/Bosses/Blueprints/BP_FightPad.BP_FightPad_C"))
  (bind _outactors_2 (`GameplayStatics.GetAllActorsOfClass` "/Game/Bosses/Blueprints/BP_Boss.BP_Boss_C"))
  (bind _outactors_3 (`GameplayStatics.GetAllActorsOfClassWithTag` "/Game/Bosses/Blueprints/BP_FightPad.BP_FightPad_C" "Boss 2"))
  (bind _outactors_4 (`GameplayStatics.GetAllActorsOfClassWithTag` "/Game/Bosses/Blueprints/BP_FightPad.BP_FightPad_C" "Boss 3"))
  (`KismetSystemLibrary.RetriggerableDelay` 0.2 :!label _label)
  (bind _output (`|GetArrayItem` _outactors_2))
  (if (== (`/Game/Bosses/Blueprints/BP_Boss.CurrentBoss` _output) 1)
    (`self.K2_TeleportTo` (`SceneComponent.K2_GetComponentLocation` (`/Game/Bosses/Blueprints/BP_FightPad.CameraPos` (`|GetArrayItem` _outactors))) _camrot)
    (goto _label)
    (elif (== (`/Game/Bosses/Blueprints/BP_Boss.CurrentBoss` _output) 2)
      (`self.K2_TeleportTo` (`SceneComponent.K2_GetComponentLocation` (`/Game/Bosses/Blueprints/BP_FightPad.CameraPos` (`|GetArrayItem` _outactors_3))) _camrot)
      (goto _label)
      (else
        (`self.K2_TeleportTo` (`SceneComponent.K2_GetComponentLocation` (`/Game/Bosses/Blueprints/BP_FightPad.CameraPos` (`|GetArrayItem` _outactors_4))) _camrot)
        (goto _label)))))

(fn `UserConstructionScript`)