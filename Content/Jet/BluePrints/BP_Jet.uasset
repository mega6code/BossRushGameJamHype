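; BP_Jet is the flipbook-animated player character, with Enhanced Input movement and a fireball attack that damages BP_Boss directly.
; FightStart freezes movement and input, shows the fighting UI and teleports Jet to a tagged or default BP_FightPad based on the current boss.
; Retriggerable-delay loops poll state to attach the camera to BP_CamPos or the spring arm, and to clear the UI and restore input once BossRef.IsAlive is false.
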(event `WhiteSMRef`
  (bind _outactors (`GameplayStatics.GetAllActorsOfClass` "/Game/Bosses/Blueprints/BP_Boss.BP_Boss_C"))
  (set `self.BossRef` (`|GetArrayItem` _outactors)))

(event `self.ReceiveBeginPlay`
  ; Starting Initialization
  (`self.WhiteSMRef`)
  (bind _asplayer_controller (cast `PlayerController` (`self.GetController`)))
  (`EnhancedInputSubsystemInterface.AddMappingContext` (pcsubsystem `EnhancedInputLocalPlayerSubsystem` _asplayer_controller) "/Game/Jet/Inputs/IMC_Jet.IMC_Jet" 0 (struct)))

(event `FightStart`
  ; Figh Start
  (set `self.IsFighting` true)
  (bind _outactors (`GameplayStatics.GetAllActorsOfClass` "/Game/Bosses/Blueprints/BP_FightPad.BP_FightPad_C"))
  (bind _outactors_2 (`GameplayStatics.GetAllActorsOfClassWithTag` "/Game/Bosses/Blueprints/BP_FightPad.BP_FightPad_C" "Boss 2"))
  (bind _outactors_3 (`GameplayStatics.GetAllActorsOfClassWithTag` "/Game/Bosses/Blueprints/BP_FightPad.BP_FightPad_C" "Boss 3"))
  (if (`/Game/Bosses/Blueprints/BP_Boss.IsAlive` (`self.BossRef`))
    (`CharacterMovementComponent.DisableMovement` (`self.CharacterMovement`) :!label _label)
    (`self.DisableInput` null)
    (`PaperFlipbookComponent.SetFlipbook` (`self.Sprite`) "/Game/Jet/Sprites/FB_Idling.FB_Idling")
    (`self.Move Camera`)
    (bind _returnvalue (`|CreateWidget` "/Game/UI/Blueprints/WB_FightingUI.WB_FightingUI_C"))
    (`UserWidget.AddToViewport` _returnvalue 0)
    (if (== (`/Game/Bosses/Blueprints/BP_Boss.CurrentBoss` (`self.BossRef`)) 0)
      (`self.K2_TeleportTo` (`SceneComponent.K2_GetComponentLocation` (`/Game/Bosses/Blueprints/BP_FightPad.PlayerPos` (`|GetArrayItem` _outactors))) (struct) :!label _label_2)
      (elif (== (`/Game/Bosses/Blueprints/BP_Boss.CurrentBoss` (`self.BossRef`)) 1)
        (`self.K2_TeleportTo` (`SceneComponent.K2_GetComponentLocation` (`/Game/Bosses/Blueprints/BP_FightPad.PlayerPos` (`|GetArrayItem` _outactors_2))) (struct))
        (elif (== (`/Game/Bosses/Blueprints/BP_Boss.CurrentBoss` (`self.BossRef`)) 3)
          (goto _label_2)
          (else
            (`self.K2_TeleportTo` (`SceneComponent.K2_GetComponentLocation` (`/Game/Bosses/Blueprints/BP_FightPad.PlayerPos` (`|GetArrayItem` _outactors_3))) (struct))))))
    (`KismetSystemLibrary.RetriggerableDelay` 0.2 :!label _label_3)
    (if (`/Game/Bosses/Blueprints/BP_Boss.IsAlive` (`self.BossRef`))
      (goto _label_3)
      (else
        (set `self.IsFighting` false)
        (bind _foundwidgets (`WidgetBlueprintLibrary.GetAllWidgetsOfClass` "/Game/UI/Blueprints/WB_FightingUI.WB_FightingUI_C"))
        (`Widget.RemoveFromParent` _foundwidgets)
        (`self.EnableInput` null)))
    (elif (`/Game/Bosses/Blueprints/BP_Boss.IsAlive2` (`self.BossRef`))
      (goto _label))))

(event `Move Camera`
  (bind _camera (`self.Camera`))
  ; Figh Start
  (bind _returnvalue (`GameplayStatics.GetActorOfClass` "/Game/Bosses/Blueprints/BP_CamPos.BP_CamPos_C"))
  (`KismetSystemLibrary.RetriggerableDelay` 0.1 :!label _label_4)
  (if (`self.IsFighting`)
    (`SceneComponent.K2_AttachToComponent` _camera (`/Game/Bosses/Blueprints/BP_CamPos.Arrow` _returnvalue) "None" "KeepRelative" "KeepRelative" "KeepRelative" true)
    (goto _label_4)
    (else
      (`SceneComponent.K2_AttachToComponent` _camera (`self.SpringArm`) "None" "KeepRelative" "KeepRelative" "KeepRelative" true)
      (goto _label_4))))

(event `EnhancedInput|/Game/Jet/Inputs/IA_MoveAD`
  (params (ActionValue :type "Float (double-precision)") (ElapsedSeconds :type "Float (double-precision)") (TriggeredSeconds :type "Float (double-precision)") (InputAction :type "InputAction Object Reference" :default "/Game/Jet/Inputs/IA_MoveAD.IA_MoveAD"))
  ; Moving
  (:`Triggered`
    (`self.AddMovementInput` (1.0 0.0 0.0) ActionValue)
    (`PaperFlipbookComponent.SetFlipbook` (`self.Sprite`) "/Game/Jet/Sprites/FB_Running.FB_Running" :!label _label_5)
    (`Controller.SetControlRotation` (`self.GetController`) (select `bool` (> ActionValue 0.0) :`false` (`KismetMathLibrary.MakeRotator` 0.0 0.0 180.0) :`true` (`KismetMathLibrary.MakeRotator` 0.0 0.0 0.0))))
  (:`Completed`
    (`PaperFlipbookComponent.SetFlipbook` (`self.Sprite`) "/Game/Jet/Sprites/FB_Idling.FB_Idling" :!label _label_6)))

(event `Shoot Fireball`
  (bind _sprite (`self.Sprite`))
  (set `self.IsAttacking` true)
  (`PaperFlipbookComponent.SetFlipbook` _sprite "/Game/Jet/Sprites/FB_FireballAttack.FB_FireballAttack")
  (`PaperFlipbookComponent.SetLooping` _sprite false)
  (`GameplayStatics.ApplyDamage` (`self.BossRef`) 10.0)
  (set `self.IsAttacking` false))

(event `EnhancedInput|/Game/Jet/Inputs/IA_MoveWS`
  (params (ActionValue :type "Float (double-precision)") (ElapsedSeconds :type "Float (double-precision)") (TriggeredSeconds :type "Float (double-precision)") (InputAction :type "InputAction Object Reference" :default "/Game/Jet/Inputs/IA_MoveWS.IA_MoveWS"))
  ; Moving
  (:`Triggered`
    (`self.AddMovementInput` (0.0 -1.0 0.0) ActionValue)
    (goto _label_5))
  (:`Completed`
    (goto _label_6)))

(event `self.Sprite.OnFinishedPlaying`
  (`PaperFlipbookComponent.SetFlipbook` (`self.Sprite`) "/Game/Jet/Sprites/FB_Idling.FB_Idling")
  (`PaperFlipbookComponent.SetLooping` (`self.Sprite`) true)
  (if (not (`PaperFlipbookComponent.IsPlaying` (`self.Sprite`)))
    (`PaperFlipbookComponent.Play` (`self.Sprite`))))

(fn `UserConstructionScript`)